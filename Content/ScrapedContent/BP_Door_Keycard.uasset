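; Sliding door actor, apparently meant to be keycard-gated for BP_Player, with the keycard check left unwired.
; E plays the DoorAnimation timeline to slide DoorMesh; the player leaving the Box trigger reverses it and disables input.
; Box entry only casts to BP_Player: the EnableInput call is disconnected and the Keycards value is unused.
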(event `self.Box.OnComponentBeginOverlap`
  (params (OverlappedComponent :type "PrimitiveComponent Object Reference") (OtherActor :type "Actor Object Reference") (OtherComp :type "PrimitiveComponent Object Reference") (OtherBodyIndex :type Integer) (bFromSweep :type Boolean) (SweepResult :type "HitResult Structure (by ref)"))
  (bind _asbp_player (cast `/Game/ThirdPerson/Blueprints/BP_Player` OtherActor)))

(event `self.Box.OnComponentEndOverlap`
  (params (OverlappedComponent :type "PrimitiveComponent Object Reference") (OtherActor :type "Actor Object Reference") (OtherComp :type "PrimitiveComponent Object Reference") (OtherBodyIndex :type Integer))
  (cast `/Game/ThirdPerson/Blueprints/BP_Player` OtherActor)
  (`self.DisableInput` (`GameplayStatics.GetPlayerController` 0))
  (bind (_direction _doorsliding) (`Timeline|DoorAnimation` :!via `Reverse` :!label _label)
    (:`Update`
      (`SceneComponent.K2_SetRelativeLocationAndRotation` :`self` (`self.DoorMesh`) :`NewLocation` _doorsliding))))

(event `Key|E`
  (params (Key :type "Key Structure"))
  (:`Pressed`
    (goto _label)))

(fn `UserConstructionScript`)