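; BP_CollapsingConstructionLift is a construction lift that shakes and then collapses when the player enters its trigger box.
; The Shaking timeline moves the lift mesh between the Arrow and LiftEndLocation positions, with a 3-second Delay on its update leading to the Collapse timeline.
; Collapse lerps the mesh from its current location toward FallPoint.
; A separate Box overlap by the player reloads the current level.
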(event `self.PlayerInsideCollisonTriggerBox.OnComponentBeginOverlap`
  (params (OverlappedComponent :type "PrimitiveComponent Object Reference") (OtherActor :type "Actor Object Reference") (OtherComp :type "PrimitiveComponent Object Reference") (OtherBodyIndex :type Integer) (bFromSweep :type Boolean) (SweepResult :type "HitResult Structure (by ref)"))
  (cast `/Game/ThirdPerson/Blueprints/BP_Player` OtherActor)
  (bind (_direction _shaking) (`Timeline|Shaking`)
    (:`Update`
      (`SceneComponent.K2_SetWorldLocation` (`self.LiftMesh`) (`KismetMathLibrary.VLerp` (`SceneComponent.K2_GetComponentLocation` (`self.Arrow`)) (`SceneComponent.K2_GetComponentLocation` (`self.LiftEndLocation`)) _shaking) false false)
      (`KismetSystemLibrary.Delay` 3.0)
      (bind (_direction_2 _collapse) (`Timeline|Collapse`)
        (:`Update`
          (`SceneComponent.K2_SetWorldLocation` (`self.LiftMesh`) (`KismetMathLibrary.VLerp` (`SceneComponent.K2_GetComponentLocation` (`self.LiftMesh`)) (`SceneComponent.K2_GetComponentLocation` (`self.FallPoint`)) _collapse) false false))))))

(event `self.Box.OnComponentBeginOverlap`
  (params (OverlappedComponent :type "PrimitiveComponent Object Reference") (OtherActor :type "Actor Object Reference") (OtherComp :type "PrimitiveComponent Object Reference") (OtherBodyIndex :type Integer) (bFromSweep :type Boolean) (SweepResult :type "HitResult Structure (by ref)"))
  (cast `/Game/ThirdPerson/Blueprints/BP_Player` OtherActor)
  (bind _returnvalue (`GameplayStatics.GetCurrentLevelName` true))
  (`GameplayStatics.OpenLevel` (`KismetStringLibrary.Conv_StringToName` _returnvalue)))

(fn `UserConstructionScript`)