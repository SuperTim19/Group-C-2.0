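; GM_Vagabond is a game mode Blueprint, judging by its name, that runs a simple countdown timer.
; While StartTimer is true, Tick passes through a one-second Delay, which throttles the per-frame calls, then decrements TimerSeconds and prints it.
; StartTimer clears once the count is no longer above zero.
; Nothing in this file starts the timer or acts on its end.
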(event `self.ReceiveTick`
  (params (DeltaSeconds :type "Float (single-precision)"))
  (if (`self.StartTimer?`)
    (if (> (`self.Timer_Seconds`) 0)
      (`KismetSystemLibrary.Delay` 1.0)
      (bind _result (`/Engine/EditorBlueprintResources/StandardMacros.DecrementInt` (`self.Timer_Seconds`))
        (:`  `
          (`KismetSystemLibrary.PrintString` (`KismetStringLibrary.Concat_StrStr` "Timer: " (`KismetStringLibrary.Conv_IntToString` _result)))))
      (else
        (set `self.StartTimer?` false)))))

(fn `UserConstructionScript`)