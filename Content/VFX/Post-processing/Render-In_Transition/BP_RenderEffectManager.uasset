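; BP_RenderEffectManager drives a render-in transition effect centered on the player character, triggered at BeginPlay.
; Each StartTransition event writes the player mesh's world location to the Position parameter of the MP_TransitionParameters collection.
; A FlipFlop alternates between playing and reversing a timeline whose Alpha feeds the collection's Radius, expanding or retracting the effect.
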(event `self.ReceiveBeginPlay`
  (`self.Start Transition (Event)`))

(event `Start Transition (Event)`
  (`KismetMaterialLibrary.SetVectorParameterValue` "/Game/VFX/Post-processing/Render-In_Transition/MP_TransitionParameters.MP_TransitionParameters" "Position" (`KismetMathLibrary.Conv_VectorToLinearColor` (`SceneComponent.K2_GetComponentLocation` (`Character.Mesh` (cast `/Game/ThirdPerson/Blueprints/BP_Player` (`GameplayStatics.GetPlayerCharacter` 0) :!pure true)))))
  (`/Engine/EditorBlueprintResources/StandardMacros.FlipFlop`
    (:`A`
      (bind (_direction _alpha) (`Timeline|Timeline` :!label _label)
        (:`Update`
          (`KismetMaterialLibrary.SetScalarParameterValue` "/Game/VFX/Post-processing/Render-In_Transition/MP_TransitionParameters.MP_TransitionParameters" "Radius" _alpha))))
    (:`B`
      (goto _label :!via `Reverse`))))

(fn `UserConstructionScript`)