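; BP_CheckpointSystem is a checkpoint actor that updates the player's respawn point when they pass through its trigger.
; On trigger overlap it casts to BP_Player and, through a DoOnce, copies the RespawnPoint component's world transform into the player's RespawnLoc.
; The same one-time activation then spawns NS_Checkpoint Niagara effects at two emitter location components as visual feedback.
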(event `self.Trigger.OnComponentBeginOverlap`
  (params (OverlappedComponent :type "PrimitiveComponent Object Reference") (OtherActor :type "Actor Object Reference") (OtherComp :type "PrimitiveComponent Object Reference") (OtherBodyIndex :type Integer) (bFromSweep :type Boolean) (SweepResult :type "HitResult Structure (by ref)"))
  ;[1 1 1] When the player passes through the trigger, their respawn will be set to match the respawn point's
  (bind _asbp_player (cast `/Game/ThirdPerson/Blueprints/BP_Player` OtherActor))
  (bind _output_get (set `self.As BP Player` _asbp_player))
  (`/Engine/EditorBlueprintResources/StandardMacros.DoOnce` false
    (:`Completed`
      (`|ExecutionSequence`
        (:`then_0`
          ;;[1 0.8148 0] Data Communicaton
          (set `/Game/ThirdPerson/Blueprints/BP_Player.RespawnLoc` (`SceneComponent.K2_GetComponentToWorld` (`self.Respawn Point`)) _output_get))
        (:`then_1`
          ;;[0 1 0.9747] Visual Effects And Animations
          (`NiagaraFunctionLibrary.SpawnSystemAtLocation` "/Game/VFX/NS_Checkpoint.NS_Checkpoint" (`SceneComponent.K2_GetComponentLocation` (`self.ParticleEmitterLoc1`)))
          (`NiagaraFunctionLibrary.SpawnSystemAtLocation` "/Game/VFX/NS_Checkpoint.NS_Checkpoint" (`SceneComponent.K2_GetComponentLocation` (`self.ParticleEmitterLoc2`))))))))

(fn `UserConstructionScript`)