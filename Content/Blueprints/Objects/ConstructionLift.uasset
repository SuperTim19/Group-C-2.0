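; Construction lift that rises while the player character is inside its trigger box and returns when they leave.
; Box overlaps play or reverse the MoveUp timeline, whose alpha lerps the lift mesh's world location between the actor's BeginPlay position and the LiftEndLocation component.
; Each timeline update also prints the alpha and computed position for debugging, and an unused relative-location variant of the move remains disconnected.
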(event `self.ReceiveBeginPlay`
  (set `self.StartPoint` (`self.K2_GetActorLocation`)))

(event `self.PlayerInsideCollisonTriggerBox.OnComponentBeginOverlap`
  (params (OverlappedComponent :type "PrimitiveComponent Object Reference") (OtherActor :type "Actor Object Reference") (OtherComp :type "PrimitiveComponent Object Reference") (OtherBodyIndex :type Integer) (bFromSweep :type Boolean) (SweepResult :type "HitResult Structure (by ref)"))
  (cast `/Game/ThirdPerson/Blueprints/BP_ThirdPersonCharacter` OtherActor)
  (bind (_direction _move_up) (`Timeline|Move Up` :!label _label)
    (:`Update`
      (bind _returnvalue (`KismetMathLibrary.VLerp` (`self.StartPoint`) (`SceneComponent.K2_GetComponentLocation` (`self.LiftEndLocation`)) _move_up))
      (`SceneComponent.K2_SetWorldLocation` (`self.LiftMesh`) _returnvalue false false)
      (`KismetSystemLibrary.PrintString` (`KismetStringLibrary.Concat_StrStr` (`KismetStringLibrary.Conv_DoubleToString` _move_up) (`KismetStringLibrary.Conv_VectorToString` _returnvalue))))))

(event `self.PlayerInsideCollisonTriggerBox.OnComponentEndOverlap`
  (params (OverlappedComponent :type "PrimitiveComponent Object Reference") (OtherActor :type "Actor Object Reference") (OtherComp :type "PrimitiveComponent Object Reference") (OtherBodyIndex :type Integer))
  (cast `/Game/ThirdPerson/Blueprints/BP_ThirdPersonCharacter` OtherActor)
  (goto _label :!via `Reverse`))

(fn `UserConstructionScript`)