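; BP_SwitchButton is a pressure button that the player triggers by overlapping its trigger volume, sending a door interaction message.
; Overlap by BP_Player plays the PressIn timeline from the start.
; Only when the timeline finishes does it lower the button mesh via a lerp from its current location, then call InteractionDoor1Message.
; Nothing resets the button or blocks repeat presses, so the offset can accumulate.
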(event `self.ReceiveBeginPlay`)

(event `self.Trigger.OnComponentBeginOverlap`
  (params (OverlappedComponent :type "PrimitiveComponent Object Reference") (OtherActor :type "Actor Object Reference") (OtherComp :type "PrimitiveComponent Object Reference") (OtherBodyIndex :type Integer) (bFromSweep :type Boolean) (SweepResult :type "HitResult Structure (by ref)"))
  (bind _msh_button (`self.Msh_Button`))
  (bind (_returnvalue_x _returnvalue_y _returnvalue_z) (`KismetMathLibrary.BreakVector` (`SceneComponent.K2_GetComponentLocation` _msh_button)))
  (cast `/Game/ThirdPerson/Blueprints/BP_Player` OtherActor)
  (bind (_direction _alpha) (`Timeline|PressIn` :!via `PlayFromStart`)
    (:`Finished`
      (`SceneComponent.K2_SetWorldLocation` (`self.Msh_Button`) (`KismetMathLibrary.VLerp` (`SceneComponent.K2_GetComponentLocation` _msh_button) (`KismetMathLibrary.MakeVector` _returnvalue_x _returnvalue_y (- _returnvalue_z 13.0)) _alpha) false false)
      (message `/Game/Blueprints/Objects/Switch/BPI_ButtonInteraction.Interaction Door 1`))))

(fn `UserConstructionScript`)