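; Wrecking ball obstacle that swings on its cable from the moment play begins.
; The XAxis flag picks which rotation axis receives the fixed swing angle.
; The BallSwing timeline drives a rotator lerp that sets the Cable's world rotation each update.
; A Move timeline for lerping Object between StartPoint and EndPoint is left unconnected and never runs.
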(event `self.ReceiveBeginPlay`
  (set `self.StartPoint` (`self.K2_GetActorLocation`))
  (if (`self.X Axis?`)
    (set `self.Swing Angle` (struct :`Roll` -70.0))
    (bind (_direction _swing) (`Timeline|Ball Swing` :!label _label)
      (:`Update`
        (`SceneComponent.K2_SetWorldRotation` (`self.Cable`) (`KismetMathLibrary.RLerp` (struct) (`self.Swing Angle`) _swing) false false)))
    (else
      (set `self.Swing Angle` (struct :`Pitch` -70.0))
      (goto _label))))

(fn `UserConstructionScript`)