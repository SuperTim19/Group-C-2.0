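; BP_MoveDropLift is a lift that carries its mesh upward when the player enters its trigger, then drops it.
; The MoveUp timeline, played at LiftSpeed, lerps the mesh from the actor's starting location to LiftEndLocation.
; On reaching that point, Falling waits briefly, then a second timeline lerps the mesh toward FallPoint from its continually updated position, compounding the motion.
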(event `self.ReceiveBeginPlay`
  (set `self.StartPoint` (`self.K2_GetActorLocation`)))

(event `self.PlayerInsideCollisonTriggerBox.OnComponentBeginOverlap`
  (params (OverlappedComponent :type "PrimitiveComponent Object Reference") (OtherActor :type "Actor Object Reference") (OtherComp :type "PrimitiveComponent Object Reference") (OtherBodyIndex :type Integer) (bFromSweep :type Boolean) (SweepResult :type "HitResult Structure (by ref)"))
  (cast `/Game/ThirdPerson/Blueprints/BP_Player` OtherActor)
  (`TimelineComponent.SetPlayRate` (`self.Move Up`) (`self.Lift Speed`))
  (bind (_direction _move_up) (`Timeline|Move Up`)
    (:`Update`
      (bind _returnvalue (`KismetMathLibrary.VLerp` (`self.StartPoint`) (`SceneComponent.K2_GetComponentLocation` (`self.LiftEndLocation`)) _move_up))
      (`SceneComponent.K2_SetWorldLocation` (`self.LiftMesh`) _returnvalue false false)
      (if (== (`SceneComponent.K2_GetComponentLocation` (`self.LiftEndLocation`)) _returnvalue)
        (`self.Falling`)))))

(event `Falling`
  (`KismetSystemLibrary.Delay` 3.0)
  (bind (_direction _collapse) (`Timeline|Timeline`)
    (:`Update`
      (`SceneComponent.K2_SetWorldLocation` (`self.LiftMesh`) (`KismetMathLibrary.VLerp` (`SceneComponent.K2_GetComponentLocation` (`self.LiftMesh`)) (`SceneComponent.K2_GetComponentLocation` (`self.FallPoint`)) _collapse) false false))))

(fn `UserConstructionScript`)