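; BP_TeleportTrap is a trap object that teleports the player when they overlap its box.
; On overlap it disables input and plays a timeline that squashes the player mesh to zero width while stretching it vertically.
; After a short delay it calls TeleportPlayer on BP_Player, while a second timeline plays in reverse to restore the mesh scale and then re-enables input.
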(event `self.Box.OnComponentBeginOverlap`
  (params (OverlappedComponent :type "PrimitiveComponent Object Reference") (OtherActor :type "Actor Object Reference") (OtherComp :type "PrimitiveComponent Object Reference") (OtherBodyIndex :type Integer) (bFromSweep :type Boolean) (SweepResult :type "HitResult Structure (by ref)"))
  (bind _asbp_player (cast `/Game/ThirdPerson/Blueprints/BP_Player` OtherActor))
  ;[1 1 1] Disables the player's movement while the animation is playing
  (`self.DisableInput` _asbp_player (`GameplayStatics.GetPlayerController` 0))
  ;[1 1 1] Animation for begining teleport
  (bind (_direction _deform_alpha) (`Timeline|TeleportDeform` :!via `PlayFromStart`)
    (:`Update`
      (bind _mesh (`Character.Mesh` _asbp_player))
      (`SceneComponent.SetWorldScale3D` _mesh (`KismetMathLibrary.VLerp` (1.0 1.0 1.0) (0.0 0.0 1.75) _deform_alpha)))
    (:`Finished`
      ;[1 1 1] Animation and Sequence for Ending the Teleport
      (`KismetSystemLibrary.Delay` 0.5)
      (`|ExecutionSequence`
        (:`then_0`
          (`/Game/ThirdPerson/Blueprints/BP_Player.Teleport Player` _asbp_player))
        (:`then_1`
          (bind (_direction_2 _deform_alpha_2) (`Timeline|Timeline` :!via `ReverseFromEnd`)
            (:`Update`
              (`SceneComponent.SetWorldScale3D` _mesh (`KismetMathLibrary.VLerp` (1.0 1.0 1.0) (0.0 0.0 1.75) _deform_alpha_2)))
            (:`Finished`
              (`self.EnableInput` _asbp_player (`GameplayStatics.GetPlayerController` 0)))))))))

(fn `UserConstructionScript`)