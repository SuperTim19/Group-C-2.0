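; BP_CogBox is a one-shot pickup that awards cogs and extra time and bounces the player upward.
; On Box overlap with BP_Player, it adds its stored values to the game mode's CogsToAdd and TimeLeft, launches the player, then destroys itself.
; It starts a looping IncreaseCogs timer by name on the game mode, so the count-up is independent of the destroyed box.
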(event `self.ReceiveBeginPlay`
  (`|ExecutionSequence`
    (:`then_0`
      (bind _asbp_player (cast `/Game/ThirdPerson/Blueprints/BP_Player` (`GameplayStatics.GetPlayerCharacter` 0)))
      (set `self.Player Ref` _asbp_player))
    (:`then_1`
      (bind _asbp_third_person_game_mode (cast `/Game/ThirdPerson/Blueprints/BP_ThirdPersonGameMode` (`GameplayStatics.GetGameMode`)))
      (set `self.Gamemode Ref` _asbp_third_person_game_mode))))

(event `self.Box.OnComponentBeginOverlap`
  (params (OverlappedComponent :type "PrimitiveComponent Object Reference") (OtherActor :type "Actor Object Reference") (OtherComp :type "PrimitiveComponent Object Reference") (OtherBodyIndex :type Integer) (bFromSweep :type Boolean) (SweepResult :type "HitResult Structure (by ref)"))
  (bind _gamemode_ref (`self.Gamemode Ref`))
  (bind _gamemode_ref_2 (`self.Gamemode Ref`))
  (bind _asbp_player (cast `/Game/ThirdPerson/Blueprints/BP_Player` OtherActor))
  (set `/Game/ThirdPerson/Blueprints/BP_ThirdPersonGameMode.CogsToAdd` (+ (`/Game/ThirdPerson/Blueprints/BP_ThirdPersonGameMode.CogsToAdd` _gamemode_ref) (`self.StoredCogs`)) _gamemode_ref)
  (`KismetSystemLibrary.K2_SetTimer` (`self.Gamemode Ref`) "IncreaseCogs" 0.4 true)
  (bind _output_get (set `/Game/ThirdPerson/Blueprints/BP_ThirdPersonGameMode.TimeLeft` (+ (`/Game/ThirdPerson/Blueprints/BP_ThirdPersonGameMode.TimeLeft` _gamemode_ref_2) (`self.Timer_New_Time`)) _gamemode_ref_2))
  (`KismetSystemLibrary.PrintString` (`KismetStringLibrary.Conv_DoubleToString` _output_get))
  (`Character.LaunchCharacter` _asbp_player (0.0 0.0 2500.0) false false)
  (`self.K2_DestroyActor`))

(fn `UserConstructionScript`)