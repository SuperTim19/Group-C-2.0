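; BP_RocketLauncherBullet is a rocket launcher projectile that restarts the current level when its box overlaps BP_Player.
; Each Tick finds a BP_RocketLauncher in the level and reads IsPlayerLeft to move along negative or positive world X.
; Movement is a fixed, unswept step per frame, not scaled by delta time, and a Delay in Tick destroys the bullet after ten seconds.
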(event `self.ReceiveTick`
  (params (DeltaSeconds :type "Float (single-precision)"))
  (bind _returnvalue (`self.K2_GetActorLocation`))
  (bind _returnvalue_2 (`self.K2_GetActorLocation`))
  (bind _returnvalue_3 (`GameplayStatics.GetActorOfClass` "/Game/Blueprints/Objects/BP_RocketLauncher.BP_RocketLauncher_C"))
  (if (`/Game/Blueprints/Objects/BP_RocketLauncher.IsPlayerLeft?` _returnvalue_3)
    (`self.K2_AddActorWorldOffset` (* (`KismetMathLibrary.GetDirectionUnitVector` _returnvalue_2 (- _returnvalue_2 (100.0 0.0 0.0))) 5))
    (`KismetSystemLibrary.Delay` 10.0)
    (`self.K2_DestroyActor`)
    (else
      (`self.K2_AddActorWorldOffset` (* (`KismetMathLibrary.GetDirectionUnitVector` _returnvalue (+ _returnvalue (100.0 0.0 0.0))) 5))
      (`KismetSystemLibrary.Delay` 10.0)
      (`self.K2_DestroyActor`))))

(event `self.Box.OnComponentBeginOverlap`
  (params (OverlappedComponent :type "PrimitiveComponent Object Reference") (OtherActor :type "Actor Object Reference") (OtherComp :type "PrimitiveComponent Object Reference") (OtherBodyIndex :type Integer) (bFromSweep :type Boolean) (SweepResult :type "HitResult Structure (by ref)"))
  (cast `/Game/ThirdPerson/Blueprints/BP_Player` OtherActor)
  (bind _returnvalue (`GameplayStatics.GetCurrentLevelName` true))
  (`GameplayStatics.OpenLevel` (`KismetStringLibrary.Conv_StringToName` _returnvalue)))

(fn `UserConstructionScript`)