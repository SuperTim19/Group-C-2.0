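; Teleporter that sends the player to its progression point when they enter its box, with a dissolve effect.
; Overlap disables input, zeroes velocity and gravity, swaps Sasha's materials to Dematerialize and fades the "Amount" parameter through a timeline.
; After fixed delays it moves the player, restoring input and gravity immediately while a second timeline reverses the dissolve, then reapplies the original materials.
; Tick continuously spins the generator flaps submesh.
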(event `BeginDematerialize`
  (bind (_direction _alpha) (`Timeline|FadeOut`)
    (:`Update`
      (`MeshComponent.SetScalarParameterValueOnMaterials` (`/Game/ThirdPerson/Blueprints/BP_Player.Sasha_Mesh` (`self.PlayerRef`)) "Amount" (`KismetMathLibrary.Lerp` 0.0 1.0 _alpha)))))

(event `Materialize`
  (bind (_direction _alpha) (`Timeline|Timeline_0` :!via `PlayFromStart`)
    (:`Update`
      (`MeshComponent.SetScalarParameterValueOnMaterials` (`/Game/ThirdPerson/Blueprints/BP_Player.Sasha_Mesh` (`self.PlayerRef`)) "Amount" (`KismetMathLibrary.Lerp` 1.0 0.0 _alpha)))))

(event `self.Box.OnComponentBeginOverlap`
  (params (OverlappedComponent :type "PrimitiveComponent Object Reference") (OtherActor :type "Actor Object Reference") (OtherComp :type "PrimitiveComponent Object Reference") (OtherBodyIndex :type Integer) (bFromSweep :type Boolean) (SweepResult :type "HitResult Structure (by ref)"))
  (bind _asbp_player (cast `/Game/ThirdPerson/Blueprints/BP_Player` OtherActor))
  ;[1 1 1] Disables the player's movement while the animation is playing
  (bind _ascc_player_controller (cast `/Game/ThirdPerson/Blueprints/CC_PlayerController` (`GameplayStatics.GetPlayerController` 0)))
  (`/Game/ThirdPerson/Blueprints/CC_PlayerController.Disable Input (New)` _ascc_player_controller)
  (`self.FreezePlayer`)
  (`self.BeginTeleportEffect`)
  (`KismetSystemLibrary.Delay` 2.5)
  ;[1 1 1] Animation and Sequence for Ending the Teleport
  (`KismetSystemLibrary.Delay` 0.5)
  (`|ExecutionSequence`
    (:`then_0`
      (`self.TeleportPlayer`))
    (:`then_1`
      (`self.Materialize`)
      (`KismetSystemLibrary.Delay` 2.0)
      (`self.FinishTeleportEffect`))
    (:`then_2`
      (`/Game/ThirdPerson/Blueprints/CC_PlayerController.Eable Input (New)` _ascc_player_controller)
      (`self.UnfreezePlayer`))))

(event `self.ReceiveBeginPlay`
  (bind _asbp_player (cast `/Game/ThirdPerson/Blueprints/BP_Player` (`GameplayStatics.GetPlayerCharacter` 0)))
  (set `self.PlayerRef` _asbp_player))

(event `self.ReceiveTick`
  (params (DeltaSeconds :type "Float (single-precision)"))
  (bind (_returnvalue_roll _returnvalue_pitch _returnvalue_yaw) (`KismetMathLibrary.BreakRotator` (`SceneComponent.K2_GetComponentRotation` (`self.Submesh`))))
  ;[0 1 0.1101] Animates the generator flaps around in a loop
  (bind _result (`/Engine/EditorBlueprintResources/StandardMacros.IncrementFloat` _returnvalue_yaw)
    (:`  `
      (`SceneComponent.K2_SetWorldRotation` (`self.Submesh`) (`KismetMathLibrary.MakeRotator` 0.0 0.0 _result) false false))))

(fn `BeginTeleportEffect`
  (`|ExecutionSequence`
    (:`then_0`
      (`PrimitiveComponent.SetMaterial` (`/Game/ThirdPerson/Blueprints/BP_Player.Sasha_Mesh` (`self.PlayerRef`)) 0 (`self.Dematerialize`)))
    (:`then_1`
      (`PrimitiveComponent.SetMaterial` (`/Game/ThirdPerson/Blueprints/BP_Player.Sasha_Mesh` (`self.PlayerRef`)) 1 (`self.Dematerialize`)))
    (:`then_2`
      (`PrimitiveComponent.SetMaterial` (`/Game/ThirdPerson/Blueprints/BP_Player.Sasha_Mesh` (`self.PlayerRef`)) 2 (`self.Dematerialize`)))
    (:`then_3`
      (`PrimitiveComponent.SetMaterial` (`/Game/ThirdPerson/Blueprints/BP_Player.Sasha_Mesh` (`self.PlayerRef`)) 3 (`self.Dematerialize`))
      (`self.BeginDematerialize`))))

(fn `FinishTeleportEffect`
  (`|ExecutionSequence`
    (:`then_0`
      (`PrimitiveComponent.SetMaterial` (`/Game/ThirdPerson/Blueprints/BP_Player.Sasha_Mesh` (`self.PlayerRef`)) 0 "/Game/Materials/Sasha/M_SashaBody.M_SashaBody"))
    (:`then_1`
      (`PrimitiveComponent.SetMaterial` (`/Game/ThirdPerson/Blueprints/BP_Player.Sasha_Mesh` (`self.PlayerRef`)) 1 "/Game/Materials/Sasha/M_SashaBlade.M_SashaBlade"))
    (:`then_2`
      (`PrimitiveComponent.SetMaterial` (`/Game/ThirdPerson/Blueprints/BP_Player.Sasha_Mesh` (`self.PlayerRef`)) 2 "/Game/Materials/Sasha/M_SashaVisor.M_SashaVisor"))
    (:`then_3`
      (`PrimitiveComponent.SetMaterial` (`/Game/ThirdPerson/Blueprints/BP_Player.Sasha_Mesh` (`self.PlayerRef`)) 3 "/Game/Materials/Sasha/M_SashaGun.M_SashaGun"))))

(fn `FreezePlayer`
  (bind _charactermovement (`Character.CharacterMovement` (`self.PlayerRef`)))
  (set `MovementComponent.Velocity` (0.0 0.0 0.0) _charactermovement)
  (set `CharacterMovementComponent.GravityScale` 0.0 _charactermovement))

(fn `TeleportPlayer`
  ;[0 0.2229 1] When called it will teleport the player to the "PlayerProgressionPoint"
  (bind _asbp_player (cast `/Game/ThirdPerson/Blueprints/BP_Player` (`GameplayStatics.GetPlayerCharacter` 0)))
  (`SceneComponent.K2_SetWorldLocation` (`Actor.RootComponent` _asbp_player) (`SceneComponent.K2_GetComponentLocation` (`self.PlayerProgressionPoint`)) false true))

(fn `UnfreezePlayer`
  (set `CharacterMovementComponent.GravityScale` 5.0 (`Character.CharacterMovement` (`self.PlayerRef`))))

(fn `UserConstructionScript`)