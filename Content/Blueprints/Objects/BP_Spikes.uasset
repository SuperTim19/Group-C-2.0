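; BP_Spikes is a spike hazard that restarts the current level when BP_Player overlaps its Box.
; If Movement is enabled, BeginPlay plays the SpikeMovement timeline at a raised rate.
; Each update sets MovePoint's relative location by lerping from 700 units below Cube's world location up to that location, re-reading Cube's world position every time.
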(event `self.ReceiveBeginPlay`
  (bind _returnvalue (`SceneComponent.K2_GetComponentLocation` (`self.Cube`)))
  (if (`self.Movement`)
    (`TimelineComponent.SetPlayRate` (`self.Spike Movement`) 1.5)
    (bind (_direction _move) (`Timeline|Spike Movement`)
      (:`Update`
        (`SceneComponent.K2_SetRelativeLocation` (`self.MovePoint`) (`KismetMathLibrary.VLerp` (- _returnvalue (0.0 0.0 700.0)) _returnvalue _move) false false)))))

(event `self.Box.OnComponentBeginOverlap`
  (params (OverlappedComponent :type "PrimitiveComponent Object Reference") (OtherActor :type "Actor Object Reference") (OtherComp :type "PrimitiveComponent Object Reference") (OtherBodyIndex :type Integer) (bFromSweep :type Boolean) (SweepResult :type "HitResult Structure (by ref)"))
  (cast `/Game/ThirdPerson/Blueprints/BP_Player` OtherActor)
  (bind _returnvalue (`GameplayStatics.GetCurrentLevelName` true))
  (`GameplayStatics.OpenLevel` (`KismetStringLibrary.Conv_StringToName` _returnvalue)))

(fn `UserConstructionScript`)