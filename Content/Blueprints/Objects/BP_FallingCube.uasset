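; BP_FallingCube is a platform that shakes, falls and resets after the player enters its Box trigger.
; A sped-up Shakje timeline swings the Cube between Left and Right markers, then disables Box and Platform collision.
; Timeline_0 then pulls the Cube from its current position toward FallPoint.
; A ten-second Delay on that timeline's update returns the Cube to the saved actor location and restores collision.
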(event `self.ReceiveBeginPlay`
  (set `self.StartPoint` (`self.K2_GetActorLocation`))
  (`TimelineComponent.SetPlayRate` (`self.shakje`) 3.0))

(event `self.Box.OnComponentBeginOverlap`
  (params (OverlappedComponent :type "PrimitiveComponent Object Reference") (OtherActor :type "Actor Object Reference") (OtherComp :type "PrimitiveComponent Object Reference") (OtherBodyIndex :type Integer) (bFromSweep :type Boolean) (SweepResult :type "HitResult Structure (by ref)"))
  (cast `/Game/ThirdPerson/Blueprints/BP_Player` OtherActor)
  (bind (_direction _shaking) (`Timeline|shakje` :!via `PlayFromStart`)
    (:`Update`
      (`SceneComponent.K2_SetWorldLocation` (`self.Cube`) (`KismetMathLibrary.VLerp` (`SceneComponent.K2_GetComponentLocation` (`self.Left`)) (`SceneComponent.K2_GetComponentLocation` (`self.Right`)) _shaking) false false))
    (:`Finished`
      (`PrimitiveComponent.SetCollisionEnabled` (`self.Box`) "NoCollision")
      (`PrimitiveComponent.SetCollisionEnabled` (`self.Platform`) "NoCollision")
      (bind (_direction_2 _collapse) (`Timeline|Timeline_0` :!via `PlayFromStart`)
        (:`Update`
          (`SceneComponent.K2_SetWorldLocation` (`self.Cube`) (`KismetMathLibrary.VLerp` (`SceneComponent.K2_GetComponentLocation` (`self.Cube`)) (`SceneComponent.K2_GetComponentLocation` (`self.FallPoint`)) _collapse) false false)
          (`KismetSystemLibrary.Delay` 10.0)
          (`SceneComponent.K2_SetWorldLocation` (`self.Cube`) (`self.StartPoint`) false false)
          (`PrimitiveComponent.SetCollisionEnabled` (`self.Box`) "QueryAndPhysics")
          (`PrimitiveComponent.SetCollisionEnabled` (`self.Platform`) "QueryAndPhysics"))))))

(fn `UserConstructionScript`)