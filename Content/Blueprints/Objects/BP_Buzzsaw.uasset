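; BP_Buzzsaw is a hazard that crashes and teleports the player on contact.
; BeginPlay spawns an attenuated whoosh sound at the mesh.
; A capsule hit from BP_Player passes a DoOnce with no reset, so each saw triggers once, spawning a Niagara crash effect and calling TeleportPlayer.
; Camera-tracking shutoff and knockback with lowered gravity remain as unconnected nodes, alongside debug prints in the live path.
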(event `self.ReceiveBeginPlay`
  (`GameplayStatics.SpawnSoundAtLocation` "/Game/Sound_Effects/mixkit-electric-whoosh-2596.mixkit-electric-whoosh-2596" (`SceneComponent.K2_GetComponentLocation` (`self.Mesh`)) (struct) 1.0 1.0 0.0 "/Game/Sound_Effects/WreckingBall_Atten.WreckingBall_Atten" null false))

(event `self.Capsule.OnComponentHit`
  (params (HitComponent :type "PrimitiveComponent Object Reference") (OtherActor :type "Actor Object Reference") (OtherComp :type "PrimitiveComponent Object Reference") (NormalImpulse :type "Vector Structure") (Hit :type "HitResult Structure (by ref)"))
  (`KismetSystemLibrary.PrintString` "Hello")
  (bind _asbp_player (cast `/Game/ThirdPerson/Blueprints/BP_Player` OtherActor))
  (`KismetSystemLibrary.PrintString` "Pplayer Dead")
  (set `self.As BP Player` _asbp_player)
  ;[1 1 1] Sequence handles the Death animations and post input movement
  (`/Engine/EditorBlueprintResources/StandardMacros.DoOnce` false
    (:`Completed`
      (`|ExecutionSequence`
        (:`then_0`
          (bind _capsulecomponent (`Character.CapsuleComponent` _asbp_player))
          (`NiagaraFunctionLibrary.SpawnSystemAtLocation` "/Game/VFX/Prototyping/NS_CogCrash.NS_CogCrash" (`SceneComponent.K2_GetComponentLocation` _capsulecomponent) (* (`SceneComponent.K2_GetComponentRotation` _capsulecomponent) -1.0)))
        (:`then_1`
          (bind _asbp_player_2 (cast `/Game/ThirdPerson/Blueprints/BP_Player` (`GameplayStatics.GetPlayerCharacter` 0)))
          (`/Game/ThirdPerson/Blueprints/BP_Player.Teleport Player` _asbp_player_2))))))

(fn `UserConstructionScript`)