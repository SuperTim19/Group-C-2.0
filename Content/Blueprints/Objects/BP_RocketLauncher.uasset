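; BP_RocketLauncher is a launcher hazard that fires rockets while the player is inside its left or right trigger.
; The trigger overlaps cast to BP_Player, setting whether to fire and which side the player is on.
; Tick runs through a Delay to pace shots by FireDelay, then spawns a homing or standard bullet, per IsHoming, at that side's arrow transform.
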(event `self.ReceiveTick`
  (params (DeltaSeconds :type "Float (single-precision)"))
  (bind _ishoming_ (`self.IsHoming?`))
  (bind _returnvalue (`SceneComponent.K2_GetComponentToWorld` (`self.LeftArrow`)))
  (bind _returnvalue_2 (`SceneComponent.K2_GetComponentToWorld` (`self.RightArrow`)))
  (`KismetSystemLibrary.Delay` (`self.FireDelay`))
  (if (`self.Fire`)
    (if (`self.IsPlayerLeft?`)
      (if _ishoming_
        (`|SpawnActorFromClass` "/Game/Blueprints/Objects/BP_RocketLauncherHomingBullet.BP_RocketLauncherHomingBullet_C" _returnvalue "Undefined" "OverrideRootScale" null null)
        (else
          (`|SpawnActorFromClass` "/Game/Blueprints/Objects/BP_RocketLauncherBullet.BP_RocketLauncherBullet_C" _returnvalue "Undefined" "OverrideRootScale" null null)))
      (elif _ishoming_
        (`|SpawnActorFromClass` "/Game/Blueprints/Objects/BP_RocketLauncherHomingBullet.BP_RocketLauncherHomingBullet_C" _returnvalue_2 "Undefined" "OverrideRootScale" null null)
        (else
          (`|SpawnActorFromClass` "/Game/Blueprints/Objects/BP_RocketLauncherBullet.BP_RocketLauncherBullet_C" _returnvalue_2 "Undefined" "OverrideRootScale" null null))))))

(event `self.Left Trigger.OnComponentBeginOverlap`
  (params (OverlappedComponent :type "PrimitiveComponent Object Reference") (OtherActor :type "Actor Object Reference") (OtherComp :type "PrimitiveComponent Object Reference") (OtherBodyIndex :type Integer) (bFromSweep :type Boolean) (SweepResult :type "HitResult Structure (by ref)"))
  (cast `/Game/ThirdPerson/Blueprints/BP_Player` OtherActor)
  (set `self.Fire` true)
  (set `self.IsPlayerLeft?` true))

(event `self.Left Trigger.OnComponentEndOverlap`
  (params (OverlappedComponent :type "PrimitiveComponent Object Reference") (OtherActor :type "Actor Object Reference") (OtherComp :type "PrimitiveComponent Object Reference") (OtherBodyIndex :type Integer))
  (cast `/Game/ThirdPerson/Blueprints/BP_Player` OtherActor)
  (set `self.Fire` false))

(event `self.RightTrigger.OnComponentBeginOverlap`
  (params (OverlappedComponent :type "PrimitiveComponent Object Reference") (OtherActor :type "Actor Object Reference") (OtherComp :type "PrimitiveComponent Object Reference") (OtherBodyIndex :type Integer) (bFromSweep :type Boolean) (SweepResult :type "HitResult Structure (by ref)"))
  (cast `/Game/ThirdPerson/Blueprints/BP_Player` OtherActor)
  (set `self.Fire` true)
  (set `self.IsPlayerLeft?` false))

(event `self.RightTrigger.OnComponentEndOverlap`
  (params (OverlappedComponent :type "PrimitiveComponent Object Reference") (OtherActor :type "Actor Object Reference") (OtherComp :type "PrimitiveComponent Object Reference") (OtherBodyIndex :type Integer))
  (cast `/Game/ThirdPerson/Blueprints/BP_Player` OtherActor)
  (set `self.Fire` false))

(fn `UserConstructionScript`)