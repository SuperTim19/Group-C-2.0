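; BP_RocketLauncherBullet is a rocket launcher projectile that teleports any player it hits.
; Each tick it looks up a BP_RocketLauncher and moves along its ForwardVector component at that launcher's BulletSpeed, without sweep and without delta-time scaling.
; The launcher's IsPlayerLeft flag selects between two movement branches that are identical.
; Box overlap with a BP_Player calls TeleportPlayer on that player, and the bullet persists afterward.
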(event `self.ReceiveTick`
  (params (DeltaSeconds :type "Float (single-precision)"))
  (bind _returnvalue (`GameplayStatics.GetActorOfClass` "/Game/Blueprints/Objects/Projectile/BP_RocketLauncher.BP_RocketLauncher_C"))
  (if (`/Game/Blueprints/Objects/Projectile/BP_RocketLauncher.IsPlayerLeft?` _returnvalue)
    (`self.K2_AddActorWorldOffset` (* (`SceneComponent.GetForwardVector` (`self.ForwardVector`)) (`/Game/Blueprints/Objects/Projectile/BP_RocketLauncher.Bullet Speed` _returnvalue)))
    (else
      (`self.K2_AddActorWorldOffset` (* (`SceneComponent.GetForwardVector` (`self.ForwardVector`)) (`/Game/Blueprints/Objects/Projectile/BP_RocketLauncher.Bullet Speed` _returnvalue))))))

(event `self.Box.OnComponentBeginOverlap`
  (params (OverlappedComponent :type "PrimitiveComponent Object Reference") (OtherActor :type "Actor Object Reference") (OtherComp :type "PrimitiveComponent Object Reference") (OtherBodyIndex :type Integer) (bFromSweep :type Boolean) (SweepResult :type "HitResult Structure (by ref)"))
  (bind _asbp_player (cast `/Game/ThirdPerson/Blueprints/BP_Player` OtherActor))
  (`/Game/ThirdPerson/Blueprints/BP_Player.Teleport Player` _asbp_player))

(fn `UserConstructionScript`)