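; Jump pad actor that launches the player straight up when they enter its trigger box from above.
; On Box overlap it checks that the BP_Player is higher than the box, sets its IsJumpPadding flag and plays a launch sound.
; LaunchCharacter overrides only Z velocity, keeping horizontal momentum, while the Sphere briefly squashes on Z and restores after a short delay.
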(event `self.Box.OnComponentBeginOverlap`
  (params (OverlappedComponent :type "PrimitiveComponent Object Reference") (OtherActor :type "Actor Object Reference") (OtherComp :type "PrimitiveComponent Object Reference") (OtherBodyIndex :type Integer) (bFromSweep :type Boolean) (SweepResult :type "HitResult Structure (by ref)"))
  (bind (_returnvalue_x _returnvalue_y _returnvalue_z) (`KismetMathLibrary.BreakVector` (`SceneComponent.K2_GetComponentLocation` (`self.Box`))))
  ;[0.5434 1 0.5798] Allows launch pad to eject player in Z axis velocity.
  (bind _asbp_player (cast `/Game/ThirdPerson/Blueprints/BP_Player` OtherActor))
  (bind (_returnvalue_x_2 _returnvalue_y_2 _returnvalue_z_2) (`KismetMathLibrary.BreakVector` (`self.K2_GetActorLocation` _asbp_player)))
  (if (not (<= _returnvalue_z_2 _returnvalue_z))
    (set `/Game/ThirdPerson/Blueprints/BP_Player.IsJumpPadding` true _asbp_player)
    ;;[0.4238 1 0.006914] Plays sound on impact
    (`GameplayStatics.PlaySound2D` "/Game/Sound_Effects/Launch_Pad_Cue.Launch_Pad_Cue" 1.0 1.0 0.0 null null)
    (`SceneComponent.SetWorldScale3D` (`self.Sphere`) (2.0 2.0 1.0))
    (`Character.LaunchCharacter` _asbp_player (0.0 0.0 1750.0) false true)
    (`KismetSystemLibrary.Delay` 0.1)
    (`SceneComponent.SetWorldScale3D` (`self.Sphere`) (2.0 2.0 2.0))))

(fn `UserConstructionScript`)