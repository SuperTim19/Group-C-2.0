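; BP_CogProjectile is a cog projectile actor that grows in on spawn and then flies forward.
; On BeginPlay a SizeGrow timeline scales the Projectile component from a tenth to full size, then enables movement when it finishes.
; Tick offsets the Projectile along the Arrow's forward vector by Velocity each frame, without sweep or delta-time scaling.
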(event `self.ReceiveBeginPlay`
  (bind (_direction _alpha) (`Timeline|SizeGrow` :!via `PlayFromStart`)
    (:`Update`
      (`SceneComponent.SetWorldScale3D` (`self.Projectile`) (`KismetMathLibrary.VLerp` (0.1 0.1 0.1) (1.0 1.0 1.0) _alpha)))
    (:`Finished`
      (set `self.CanMoveForward?` true))))

(event `self.ReceiveTick`
  (params (DeltaSeconds :type "Float (single-precision)"))
  ;[0 1 0.09759] Moves the actor forward each frame
  (if (`self.CanMoveForward?`)
    (`SceneComponent.K2_AddWorldOffset` (`self.Projectile`) (* (`SceneComponent.GetForwardVector` (`self.Arrow`)) (`self.Velocity`)) false false)))

(fn `UserConstructionScript`)