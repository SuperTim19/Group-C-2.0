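; BP_MrFry is a chasing enemy that pursues the player and restarts the current level when its box touches BP_Player.
; BeginPlay scales up the mesh, offsets the capsule from the player's location and plays one random 2D voice line.
; Tick moves it straight toward the player at a fixed per-frame step, without sweep or delta-time scaling.
; The debug print re-rolls the random index, so it can name a different line than the one played.
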(event `self.ReceiveBeginPlay`
  (`SceneComponent.SetRelativeScale3D` (`self.Mesh`) (10.0 10.0 4.5))
  (`SceneComponent.K2_SetRelativeLocation` (`self.CapsuleComponent`) (- (`self.K2_GetActorLocation` (`GameplayStatics.GetPlayerCharacter` 0)) (1000.0 0.0 0.0)) false false)
  (`self.Mr Fry's Voice Lines`))

(event `self.ReceiveTick`
  (params (DeltaSeconds :type "Float (single-precision)"))
  (`self.K2_AddActorWorldOffset` (* (`KismetMathLibrary.GetDirectionUnitVector` (`self.K2_GetActorLocation`) (`self.K2_GetActorLocation` (`GameplayStatics.GetPlayerCharacter` 0))) 5)))

(event `self.Box.OnComponentBeginOverlap`
  (params (OverlappedComponent :type "PrimitiveComponent Object Reference") (OtherActor :type "Actor Object Reference") (OtherComp :type "PrimitiveComponent Object Reference") (OtherBodyIndex :type Integer) (bFromSweep :type Boolean) (SweepResult :type "HitResult Structure (by ref)"))
  (cast `/Game/ThirdPerson/Blueprints/BP_Player` OtherActor)
  (bind _returnvalue (`GameplayStatics.GetCurrentLevelName` true))
  (`GameplayStatics.OpenLevel` (`KismetStringLibrary.Conv_StringToName` _returnvalue)))

(event `Mr Fry's Voice Lines`
  (bind _output (`|GetArrayItem` (`self.Lines`) (`KismetMathLibrary.RandomIntegerInRange` 0 2)))
  (bind _returnvalue (`GameplayStatics.CreateSound2D` _output 1.0 1.0 0.0 null))
  (`AudioComponent.Play` _returnvalue 0.0)
  (`KismetSystemLibrary.PrintString` (`KismetSystemLibrary.GetDisplayName` _output)))

(fn `UserConstructionScript`)