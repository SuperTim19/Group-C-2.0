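; Construction lift actor that carries LiftMesh along a spline, triggered by the player.
; Overlapping the inside trigger box plays or reverses the SplineMove timeline depending on MoveUp.
; The timeline update uses its track value as a distance along LiftSpline to set the mesh's world location.
; Leaving the exit trigger flips MoveUp and prints a debug message, so the next trip can run the opposite way.
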(event `self.PlayerInsideCollisonTriggerBox.OnComponentBeginOverlap`
  (params (OverlappedComponent :type "PrimitiveComponent Object Reference") (OtherActor :type "Actor Object Reference") (OtherComp :type "PrimitiveComponent Object Reference") (OtherBodyIndex :type Integer) (bFromSweep :type Boolean) (SweepResult :type "HitResult Structure (by ref)"))
  (cast `/Game/ThirdPerson/Blueprints/BP_Player` OtherActor)
  (if (`self.MoveUp?`)
    (`self.EventMoveUp`)
    (else
      (`self.EventMoveDown`))))

(event `EventMoveUp`
  (bind (_direction _newtrack_0) (`Timeline|SplineMove` :!label _label)
    (:`Update`
      (bind _returnvalue_location (`KismetMathLibrary.BreakTransform` (`SplineComponent.GetTransformAtDistanceAlongSpline` (`self.LiftSpline`) _newtrack_0 "World" false)))
      (`SceneComponent.K2_SetWorldLocation` (`self.LiftMesh`) _returnvalue_location false false))))

(event `EventMoveDown`
  (goto _label :!via `Reverse`))

(event `self.PlayerExitTrigger_R.OnComponentEndOverlap`
  (params (OverlappedComponent :type "PrimitiveComponent Object Reference") (OtherActor :type "Actor Object Reference") (OtherComp :type "PrimitiveComponent Object Reference") (OtherBodyIndex :type Integer))
  ;[1 1 1] Toggles Value of MoveUp/Down? when player leaves
  (cast `/Game/ThirdPerson/Blueprints/BP_Player` OtherActor)
  (set `self.MoveUp?` (not (`self.MoveUp?`)))
  (`KismetSystemLibrary.PrintString` "player has left"))

(fn `UserConstructionScript`)