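; Homing rocket projectile that chases the player and restarts the level on contact.
; Each Tick it steps toward player 0 without sweep or delta-time scaling, rotating its Cone with a look-at computed from the cone's forward vector, not its location.
; A Delay in Tick destroys it after a fixed lifetime.
; A Box overlap with BP_Player reloads the current level by name.
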(event `self.ReceiveTick`
  (params (DeltaSeconds :type "Float (single-precision)"))
  (bind _returnvalue (`self.K2_GetActorLocation` (`GameplayStatics.GetPlayerCharacter` 0)))
  (`self.K2_AddActorWorldOffset` (* (`KismetMathLibrary.GetDirectionUnitVector` (`self.K2_GetActorLocation`) _returnvalue) 2))
  (`SceneComponent.K2_SetWorldRotation` (`self.Cone`) (`KismetMathLibrary.FindLookAtRotation` (`SceneComponent.GetForwardVector` (`self.Cone`)) _returnvalue) false false)
  (`KismetSystemLibrary.Delay` 10.0)
  (`self.K2_DestroyActor`))

(event `self.Box.OnComponentBeginOverlap`
  (params (OverlappedComponent :type "PrimitiveComponent Object Reference") (OtherActor :type "Actor Object Reference") (OtherComp :type "PrimitiveComponent Object Reference") (OtherBodyIndex :type Integer) (bFromSweep :type Boolean) (SweepResult :type "HitResult Structure (by ref)"))
  (cast `/Game/ThirdPerson/Blueprints/BP_Player` OtherActor)
  (bind _returnvalue (`GameplayStatics.GetCurrentLevelName` true))
  (`GameplayStatics.OpenLevel` (`KismetStringLibrary.Conv_StringToName` _returnvalue)))

(fn `UserConstructionScript`)