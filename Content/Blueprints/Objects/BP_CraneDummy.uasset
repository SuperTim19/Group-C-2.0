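; Crane dummy actor, apparently a disconnected version of a rotating crane that holds the player in place as it turns.
; BeginPlay, Tick, overlap and spin events are empty, leaving the player tracking and delayed flip-flop rotation timeline unreachable.
; The remaining wired lock events involve a gate and setting the player's location.
; FindPlayerPOS, called only from dead logic, derives that location from a debug-drawn downward trace plus an offset.
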(event `self.ReceiveBeginPlay`)

(event `ActivateSpin`)

(event `self.PlayerCollisionBox.OnComponentBeginOverlap`
  (params (OverlappedComponent :type "PrimitiveComponent Object Reference") (OtherActor :type "Actor Object Reference") (OtherComp :type "PrimitiveComponent Object Reference") (OtherBodyIndex :type Integer) (bFromSweep :type Boolean) (SweepResult :type "HitResult Structure (by ref)")))

(event `self.PlayerCollisionBox.OnComponentEndOverlap`
  (params (OverlappedComponent :type "PrimitiveComponent Object Reference") (OtherActor :type "Actor Object Reference") (OtherComp :type "PrimitiveComponent Object Reference") (OtherBodyIndex :type Integer)))

(event `self.ReceiveTick`
  (params (DeltaSeconds :type "Float (single-precision)")))

(event `Open_CraneLock`
  (`/Engine/EditorBlueprintResources/StandardMacros.Gate` true :!via `Open`
    (:`Exit`
      (`self.CraneLock`))))

(event `Close_CraneLock`)

(event `CraneLock`
  (`self.K2_SetActorLocation` (`self.As BP Player`) (`self.PlayerLocation`) false false))

(fn `FindPlayerPOS`
  (locals (Offset :type "Vector Structure"))
  (bind _as_bp_player (`self.As BP Player`))
  (bind _returnvalue (`self.K2_GetActorLocation` _as_bp_player))
  (bind _outhit (`KismetSystemLibrary.LineTraceSingle` _returnvalue (- _returnvalue (0.0 0.0 100.0)) "TraceTypeQuery1" false (`|MakeArray` _as_bp_player :!type "Actor Object Reference") "Persistent"))
  (set `self.PlayerLocation` (+ (`.ImpactPoint` (`GameplayStatics.BreakHitResult` _outhit)) (`local.Offset`))))

(fn `UserConstructionScript`)