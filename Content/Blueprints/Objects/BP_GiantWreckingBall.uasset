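; Swinging wrecking ball obstacle that restarts the current level when the player touches it.
; On BeginPlay, the XAxis flag picks which rotation axis the swing angle uses.
; The BallSwing timeline then lerps the Cable's relative rotation toward that angle to drive the swing.
; A Sphere overlap with BP_Player reopens the current level by name.
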(event `self.ReceiveBeginPlay`
  (if (`self.X Axis?`)
    (set `self.Swing Angle` (struct :`Roll` -70.0))
    (bind (_direction _swing) (`Timeline|Ball Swing` :!label _label)
      (:`Update`
        (`SceneComponent.K2_SetRelativeRotation` (`self.Cable`) (`KismetMathLibrary.RLerp` (struct) (`self.Swing Angle`) _swing) false false)))
    (else
      (set `self.Swing Angle` (struct :`Pitch` -70.0))
      (goto _label))))

(event `self.Sphere.OnComponentBeginOverlap`
  (params (OverlappedComponent :type "PrimitiveComponent Object Reference") (OtherActor :type "Actor Object Reference") (OtherComp :type "PrimitiveComponent Object Reference") (OtherBodyIndex :type Integer) (bFromSweep :type Boolean) (SweepResult :type "HitResult Structure (by ref)"))
  (cast `/Game/ThirdPerson/Blueprints/BP_Player` OtherActor)
  (bind _returnvalue (`GameplayStatics.GetCurrentLevelName` true))
  (`GameplayStatics.OpenLevel` (`KismetStringLibrary.Conv_StringToName` _returnvalue)))

(fn `UserConstructionScript`)