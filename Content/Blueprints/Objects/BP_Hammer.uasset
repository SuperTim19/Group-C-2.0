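; BP_Hammer is a swinging hammer hazard that teleports the player when hit during its active window.
; On BeginPlay, the Swing timeline starts at SwingPlayRate and lerps the Arrow component's world rotation.
; Timeline event tracks flip the Activated flag through a FlipFlop and play the impact sound at the actor's location.
; Box overlaps with BP_Player call TeleportPlayer only while Activated is set.
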(event `self.ReceiveBeginPlay`
  (`TimelineComponent.SetPlayRate` (`self.Swing`) (`self.SwingPlayRate`))
  (bind (_direction _swing) (`Timeline|Swing`)
    (:`Update`
      (`SceneComponent.K2_SetWorldRotation` (`self.Arrow`) (`KismetMathLibrary.RLerp` (struct :`Yaw` 450.0) (struct :`Pitch` -90.0 :`Yaw` 450.0) _swing) false false))
    (:`HitActivated`
      (`/Engine/EditorBlueprintResources/StandardMacros.FlipFlop`
        (:`A`
          (set `self.activated` true))
        (:`B`
          (set `self.activated` false))))
    (:`Hit`
      (`GameplayStatics.PlaySoundAtLocation` "/Game/Sound_Effects/hammer_finals_01_Cue.hammer_finals_01_Cue" (`self.K2_GetActorLocation`) (struct) 1.0 1.0 0.0 null null null null))))

(event `self.Box.OnComponentBeginOverlap`
  (params (OverlappedComponent :type "PrimitiveComponent Object Reference") (OtherActor :type "Actor Object Reference") (OtherComp :type "PrimitiveComponent Object Reference") (OtherBodyIndex :type Integer) (bFromSweep :type Boolean) (SweepResult :type "HitResult Structure (by ref)"))
  (bind _asbp_player (cast `/Game/ThirdPerson/Blueprints/BP_Player` OtherActor))
  (if (`self.activated`)
    (`/Game/ThirdPerson/Blueprints/BP_Player.Teleport Player` _asbp_player)))

(fn `UserConstructionScript`)