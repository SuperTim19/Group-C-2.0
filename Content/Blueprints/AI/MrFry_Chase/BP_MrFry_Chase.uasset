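; BP_MrFry_Chase is the chase version of the Mr Fry AI, which grows to giant size shortly after play begins.
; A delayed, sped-up timeline scales the mesh to five times normal, then flags spawn completion and caches the player.
; Each tick afterwards draws a debug visibility trace from FirePoint to the player's capsule location offset along FirePoint's forward vector.
; The trace result is unused, and no movement logic is present.
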(event `self.ReceiveBeginPlay`
  (`KismetSystemLibrary.Delay` 3.0)
  (`TimelineComponent.SetPlayRate` (`self.MakeMrFryBig`) 2.0)
  (bind (_direction _scale) (`Timeline|MakeMrFryBig`)
    (:`Update`
      (`SceneComponent.SetRelativeScale3D` (`self.Mesh`) (`KismetMathLibrary.VLerp` (1.0 1.0 1.0) (5.0 5.0 5.0) _scale)))
    (:`Finished`
      (set `self.SpawnComplete` true)
      (bind _asbp_player (cast `/Game/ThirdPerson/Blueprints/BP_Player` (`GameplayStatics.GetPlayerCharacter` 0)))
      (set `self.Player` _asbp_player))))

(event `self.ReceiveTick`
  (params (DeltaSeconds :type "Float (single-precision)"))
  (bind _firepoint (`self.FirePoint`))
  (if (`self.SpawnComplete`)
    (`KismetSystemLibrary.LineTraceSingle` :`Start` (`SceneComponent.K2_GetComponentLocation` _firepoint) :`End` (+ (* (`KismetMathLibrary.GetForwardVector` (`SceneComponent.K2_GetComponentRotation` _firepoint)) 2000.0) (`SceneComponent.K2_GetComponentLocation` (`Character.CapsuleComponent` (`self.Player`)))) :`TraceChannel` "TraceTypeQuery1" :`DrawDebugType` "ForDuration")))

(fn `UserConstructionScript`)