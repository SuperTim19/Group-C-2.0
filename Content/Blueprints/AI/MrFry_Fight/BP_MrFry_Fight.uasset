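; BP_MrFry_Fight is the Mr Fry fight Blueprint, which fires traces at the player and teleports them on a hit.
; BeginPlay caches the player, and the self-repeating FireRate event waits a random delay, then line-traces from FirePoint toward the player's capsule.
; The loop ends if a trace hits a non-player actor, and nothing in this graph starts it.
; Debug drawing and printed trace endpoints remain active.
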(event `self.ReceiveBeginPlay`
  (bind _asbp_player (cast `/Game/ThirdPerson/Blueprints/BP_Player` (`GameplayStatics.GetPlayerCharacter` 0)))
  (set `self.Player` _asbp_player))

(event `Fire Rate`
  (bind _firepoint (`self.FirePoint`))
  (`KismetSystemLibrary.Delay` (`KismetMathLibrary.RandomFloatInRange` 2.0 10.0))
  (bind _outhit (`KismetSystemLibrary.LineTraceSingle` :`Start` (`SceneComponent.K2_GetComponentLocation` _firepoint) :`End` (+ (`KismetMathLibrary.GetForwardVector` (`SceneComponent.K2_GetComponentRotation` _firepoint)) (`SceneComponent.K2_GetComponentLocation` (`Character.CapsuleComponent` (`self.Player`)))) :`TraceChannel` "TraceTypeQuery1" :`DrawDebugType` "ForDuration"))
  (if (`GameplayStatics.BreakHitResult` _outhit)
    (bind _asbp_player (cast `/Game/ThirdPerson/Blueprints/BP_Player` (`.HitActor` (`GameplayStatics.BreakHitResult` _outhit))))
    (`/Game/ThirdPerson/Blueprints/BP_Player.Teleport Player` _asbp_player)
    (bind _returnvalue (`KismetStringLibrary.Conv_VectorToString` (`.TraceEnd` (`GameplayStatics.BreakHitResult` _outhit))))
    (`KismetSystemLibrary.PrintString` _returnvalue)
    (`self.Fire Rate`)
    (else
      (`KismetSystemLibrary.PrintString` _returnvalue)
      (`self.Fire Rate`))))

(event `self.ReceiveTick`
  (params (DeltaSeconds :type "Float (single-precision)")))

(fn `UserConstructionScript`)