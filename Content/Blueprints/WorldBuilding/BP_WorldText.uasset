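; BP_WorldText is a world text actor that bobs vertically between its starting position and a MovementOffset below it.
; The construction script applies InText to the text render component, and BeginPlay caches its location before starting the TextMovement timeline.
; The timeline's Alpha lerps the world location, while a FlipFlop on Finished alternates ReverseLoop and PlayLoop for an endless ping-pong without Tick.
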(event `Play Loop`
  (bind (_returnlocation_x _returnlocation_y _returnlocation_z) (`KismetMathLibrary.BreakVector` (`self.ReturnLocation`)))
  (bind (_direction _alpha) (`Timeline|TextMovement` :!label _label)
    (:`Update`
      (`SceneComponent.K2_SetWorldLocation` (`self.TextRender`) (`KismetMathLibrary.VLerp` (`self.ReturnLocation`) (`KismetMathLibrary.MakeVector` _returnlocation_x _returnlocation_y (- _returnlocation_z (`self.MovementOffset`))) _alpha) false false))
    (:`Finished`
      (`/Engine/EditorBlueprintResources/StandardMacros.FlipFlop`
        (:`A`
          (`self.Reverse Loop`))
        (:`B`
          (`self.Play Loop`))))))

(event `self.ReceiveBeginPlay`
  (set `self.ReturnLocation` (`SceneComponent.K2_GetComponentLocation` (`self.TextRender`)))
  (goto _label :!via `PlayFromStart`))

(event `Reverse Loop`
  (goto _label :!via `Reverse`))

(fn `UserConstructionScript`
  (`TextRenderComponent.K2_SetText` (`self.TextRender`) (`self.InText`)))