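; BP_ArrowSign is a world-building arrow sign that bobs up and down continuously from the start of play.
; BeginPlay stores the mesh's world location and starts the Hover timeline, which lerps the mesh between that position and MovementOffset units below it.
; When the timeline finishes, a FlipFlop alternates between the PlayReverse and PlayStart events, creating an endless ping-pong loop.
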(event `PlayStart`
  (bind (_startposition_x _startposition_y _startposition_z) (`KismetMathLibrary.BreakVector` (`self.StartPosition`)))
  ;[1 0 0.8869] Hover Code: Makes sign begin to hover up and down when the level begins
  (bind (_direction _alpha) (`Timeline|Hover` :!label _label)
    (:`Update`
      ;;[0.001142 1 0] Moves the arrow mesh down with a timeline
      (`SceneComponent.K2_SetWorldLocation` (`self.Mesh`) (`KismetMathLibrary.VLerp` (`self.StartPosition`) (`KismetMathLibrary.MakeVector` _startposition_x _startposition_y (- _startposition_z (`self.MovementOffset`))) _alpha) false false))
    (:`Finished`
      ;;[0 0.07514 1] Loops timeline after begin play
      (`/Engine/EditorBlueprintResources/StandardMacros.FlipFlop`
        (:`A`
          (`self.PlayReverse`))
        (:`B`
          (`self.PlayStart`))))))

(event `self.ReceiveBeginPlay`
  ;[1 0 0.8869] Hover Code: Makes sign begin to hover up and down when the level begins
  (set `self.StartPosition` (`SceneComponent.K2_GetComponentLocation` (`self.Mesh`)))
  (goto _label :!via `PlayFromStart`))

(event `PlayReverse`
  ;[1 0 0.8869] Hover Code: Makes sign begin to hover up and down when the level begins
  (goto _label :!via `Reverse`))

(fn `UserConstructionScript`)