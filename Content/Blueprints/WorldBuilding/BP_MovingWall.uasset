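; BP_MovingWall is a wall that continuously moves down and back up once the game starts.
; BeginPlay caches the Wireframe component's world location and starts the MoveWall timeline, with a timer offset for adjusting timing.
; The timeline's Alpha lerps the component between that origin and a point MovementOffset below it.
; On finish, a FlipFlop alternates reverse and forward custom events to keep the loop running.
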(event `Forward Movement`
  (bind (_returnlocation_x _returnlocation_y _returnlocation_z) (`KismetMathLibrary.BreakVector` (`self.ReturnLocation`)))
  ;[0 0.3424 1] Looping Movement Code: This code moves the wall up and down at a continous rate after the game starts. Some different variables are present to allow you to change the timing and how far down the wall will move
  ;;[0.7838 1 0.2708] Timeline that moves the wall. Custom Events are for the looping process
  (bind (_direction _alpha) (`Timeline|Move Wall` :`NewTime` (`self.TimerOffset`) :!label _label)
    (:`Update`
      ;;[0 1 0.007031] This code actually moves the actor. It uses the origin point and reduces it using an offset variable. Both are then feed into a lerp that uses the timeline's "Alpha" output
      (`SceneComponent.K2_SetWorldLocation` (`self.Wireframe`) (`KismetMathLibrary.VLerp` (`self.ReturnLocation`) (`KismetMathLibrary.MakeVector` _returnlocation_x _returnlocation_y (- _returnlocation_z (`self.MovementOffset`))) _alpha) false false))
    (:`Finished`
      ;;[0.2135 0.2135 0.2135] Moves the actor in the direction it came from when timeline finishes
      (`/Engine/EditorBlueprintResources/StandardMacros.FlipFlop`
        (:`A`
          (`self.Reverse Movement`))
        (:`B`
          (`self.Forward Movement`))))))

(event `self.ReceiveBeginPlay`
  ;[0 0.3424 1] Looping Movement Code: This code moves the wall up and down at a continous rate after the game starts. Some different variables are present to allow you to change the timing and how far down the wall will move
  ;;[1 0.803 0] Sets the origin of the actor in world space
  (set `self.ReturnLocation` (`SceneComponent.K2_GetComponentLocation` (`self.Wireframe`)))
  ;;[0.7838 1 0.2708] Timeline that moves the wall. Custom Events are for the looping process
  (`|ExecutionSequence`
    (:`then_0`
      (goto _label :!via `SetNewTime`))
    (:`then_1`
      (goto _label))))

(event `Reverse Movement`
  ;[0 0.3424 1] Looping Movement Code: This code moves the wall up and down at a continous rate after the game starts. Some different variables are present to allow you to change the timing and how far down the wall will move
  ;;[0.7838 1 0.2708] Timeline that moves the wall. Custom Events are for the looping process
  (goto _label :!via `Reverse`))

(fn `UserConstructionScript`)